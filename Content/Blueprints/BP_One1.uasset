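; BP_One1 is a shootable target that breaks apart and adds score when a BP_Bullet hits it.
; A RotatingMovement component drives the SpringArm from BeginPlay.
; The first bullet hit on the Box enables physics on the GeometryCollection, disables Box collision and calls AddScore on GM_Target_Game, with IsHit blocking repeats.
; An unconnected timeline for SpringArm pitch and an empty RotateCube function are unused leftovers.
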(event `self.ReceiveBeginPlay`
  (`MovementComponent.SetUpdatedComponent` (`self.RotatingMovement`) (`self.SpringArm`)))

(event `self.Box.OnComponentHit`
  (params (HitComponent :type "PrimitiveComponent Object Reference") (OtherActor :type "Actor Object Reference") (OtherComp :type "PrimitiveComponent Object Reference") (NormalImpulse :type "Vector Structure") (Hit :type "HitResult Structure (by ref)"))
  (cast `/Game/FirstPerson/Blueprints/BP_Bullet` OtherActor)
  (if (not (`self.IsHit?`))
    (set `self.IsHit?` true)
    (`PrimitiveComponent.SetSimulatePhysics` (`self.GeometryCollection`) true)
    (`PrimitiveComponent.SetCollisionEnabled` (`self.Box`) "NoCollision")
    (bind _asgm_target_game (cast `/Game/FirstPerson/Blueprints/GM_Target_Game` (`GameplayStatics.GetGameMode`)))
    (`/Game/FirstPerson/Blueprints/GM_Target_Game.AddScore` _asgm_target_game)))

(fn `Rotate Cube`)

(fn `UserConstructionScript`)